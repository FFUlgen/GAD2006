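; BP_NetGameState is a multiplayer game state that runs the match countdown and handles victory and restart.
; A looping one-second timer updates the local avatar's countdown widget, while authority copies the count to TimeChecker every other tick so its OnRep can resync drifting counters.
; On victory, Red avatars win and Blue lose, and a results widget shows the loss or winner's nickname until restart.
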(event EventOnCountdownOver)

(event EventBeginPlay
  (bind _returnvalue (Utilities|Time|SetTimerbyFunctionName 0 "DecreaseCounter" 1.0 true))
  (Variables|Default|SetTH_Counter _returnvalue))

(event EventOnVictory
  (for _array_element (Variables|Default|GetPlayerArray)
    (bind _asnet_player_state (Utilities|Casting|CastToNetPlayerState _array_element))
    (switch Utilities|FlowControl|Switch|SwitchonEPlayerTeam (.teamid (Variables|/Script/Labwork4.NetPlayerState|GetData _asnet_player_state))
      (:TEAM_Blue
        (Default|OnPlayerLost (.AsBP%20Net%20Avatar (Utilities|Casting|CastToBP_NetAvatar (Variables|/Script/Engine.PlayerState|GetPawnPrivate _asnet_player_state)))))
      (:TEAM_Red
        (Default|OnPlayerWon (.AsBP%20Net%20Avatar (Utilities|Casting|CastToBP_NetAvatar (Variables|/Script/Engine.PlayerState|GetPawnPrivate _asnet_player_state)))))))
  (CallFunction|ShowResultMessage))

(event EventOnRestart
  (Widget|RemovefromParent (Variables|Default|GetMessage%20Widget)))

(fn ConstructionScript)

(fn ShowResultMessage
  (bind _returnvalue (Class|NetGameState|GetPlayerStatebyIndex (Variables|Default|GetWinningPlayer)))
  (bind _returnvalue_2 (UserInterface|CreateWidget "/Game/Blueprints/UMG/W_GameResults.W_GameResults_C" 0 (select (Utilities|Enum|Equal(Enum) (.teamid (Variables|/Script/Labwork4.NetPlayerState|GetData (.AsNet%20Player%20State (Utilities|Casting|CastToNetPlayerState (Variables|/Script/Engine.Controller|GetPlayerState (Game|GetPlayerController 0)))))) "TEAM_Blue") "YOU LOSE!" (Utilities|Text|FormatText "{Name} Wins!" (.Nickname (Utilities|Struct|BreakSPlayerInfo (Variables|/Script/Labwork4.NetPlayerState|GetData _returnvalue)))))))
  (Variables|Default|SetMessage%20Widget _returnvalue_2)
  (UserInterface|Viewport|AddtoViewport (Variables|Default|GetMessage%20Widget) 0))

(fn DecreaseCounter
  (bind _result (Math|Integer|DecrementInt (Variables|Default|GetTimeCounter))
    (:%20%20
      (Networking|SwitchHasAuthority
        (:Authority
          (if (== (Math|Integer|%(Integer) _result 2) 0)
            (Variables|Default|SetTimeChecker (Variables|Default|GetTimeCounter))
            (CallFunction|SetCounter)
            (else
              (CallFunction|SetCounter))))
        (:Remote
          (CallFunction|SetCounter))))))

(fn OnRepTimeChecker
  (if (not (== (Variables|Default|GetTimeChecker) (Variables|Default|GetTimeCounter)))
    (Variables|Default|SetTimeCounter (Variables|Default|GetTimeChecker))
    (Utilities|Time|ClearandInvalidateTimerbyHandle (Variables|Default|GetTH_Counter))
    (bind _returnvalue (Utilities|Time|SetTimerbyFunctionName 0 "DecreaseCounter" 1.0 true))
    (Variables|Default|SetTH_Counter _returnvalue)
    (CallFunction|SetCounter)))

(fn SetCounter
  (bind _returnvalue (Game|GetPlayerController 0))
  (bind _returnvalue_2 (Pawn|GetControlledPawn _returnvalue))
  (Utilities|IsValid (Variables|Default|GetAs%20BP%20Net%20Avatar)
    (:Is%20Valid
      _)
    (:Is%20Not%20Valid
      (Utilities|IsValid _returnvalue_2
        (:Is%20Valid
          (bind _asbp_net_avatar (Utilities|Casting|CastToBP_NetAvatar _returnvalue_2))
          (bind _output_get (Variables|Default|SetAs%20BP%20Net%20Avatar _asbp_net_avatar))))))
  (Utilities|IsValid (Variables|/Game/Blueprints/BP_NetAvatar.BP_NetAvatar_C|GetCountdown%20Widget _output_get)
    (:Is%20Valid
      (Default|UpdateTime (Variables|/Game/Blueprints/BP_NetAvatar.BP_NetAvatar_C|GetCountdown%20Widget _output_get) (Variables|Default|GetTimeCounter))
      (if (== (Variables|Default|GetTimeCounter) 0)
        (Utilities|Time|ClearandInvalidateTimerbyHandle (Variables|Default|GetTH_Counter))
        (Widget|RemovefromParent (Variables|/Game/Blueprints/BP_NetAvatar.BP_NetAvatar_C|GetCountdown%20Widget _output_get))))))