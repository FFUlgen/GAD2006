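; BP_CharacterBase is a character base Blueprint that records recent key presses in a timestamped input buffer.
; Each AddToInputBuffer press removes entries older than 0.2 seconds inside a loop over the same array, then adds the key's display name and current time.
; A debug FlipFlop then prints the buffered names, alternating text color on each press.
; Pruning happens only on presses, and nothing in these graphs consumes the buffer beyond debug printing.
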(event EventBeginPlay)

(event EventTick
  (params (DeltaSeconds :type Float%20%28single-precision%29)))

(event Input|ActionEvents|InputActionAddToInputBuffer
  (params (Key :type Key%20Structure :default "None"))
  (bind _inputbuffer (Variables|Default|GetinputBuffer))
  (:Pressed
    (for _array_element _inputbuffer
      (if (< (.timeStamp (Utilities|Struct|BreakInputInfo _array_element)) (- (Utilities|Time|GetTimeSeconds) 0.2))
        (Utilities|Array|RemoveItem _inputbuffer _array_element)))
    (Class|FGCharacterBase|AddInputtoInputBuffer (Utilities|Struct|MakeInputInfo (Utilities|String|ToString(Text) (Class|KismetInputLibrary|KeyGetDisplayName Key true)) (Utilities|Time|GetTimeSeconds)))
    ;[1 1 1] Debug
    (Utilities|FlowControl|FlipFlop
      (:A
        (for _array_element_2 (Variables|Default|GetinputBuffer)
          (Development|PrintString (.inputName (Utilities|Struct|BreakInputInfo _array_element_2)))))
      (:B
        (for _array_element_3 (Variables|Default|GetinputBuffer)
          (Development|PrintString (.inputName (Utilities|Struct|BreakInputInfo _array_element_3)) true true "(R=1.000000,G=0.037186,B=0.000000,A=1.000000)"))))))

(fn ConstructionScript)