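; Game mode that sets up a local two-player match with fighter characters and a shared HUD.
; On BeginPlay it spawns pawns at PlayerStarts tagged P1 and P2, possessing them with player controller 0 and a newly created local player.
; Both pawns use the single CharacterClass stored in BP_FGGameInstance, either Mannequin or Mutant.
; Once both exist, it cross-links them as OtherPlayer and adds WB_HUD to the viewport.
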(event EventBeginPlay
  (bind _player2 (Variables|Default|Getplayer2))
  (bind _player1 (Variables|Default|Getplayer1))
  (bind _outactors (Actor|GetAllActorsOfClass "/Script/Engine.PlayerStart"))
  (for _array_element _outactors
    (CallFunction|SpawnPlayers _array_element))
  (if (Utilities|IsValid (Variables|Default|Getplayer1))
    (if (Utilities|IsValid (Variables|Default|Getplayer2))
      (Variables|/Script/FighterGame.FGCharacterBase|SetOtherPlayer _player1 _player2)
      (Variables|/Script/FighterGame.FGCharacterBase|SetOtherPlayer _player2 _player1)
      (bind _returnvalue (UserInterface|CreateWidget "/Game/UI/WB_HUD.WB_HUD_C" (Game|GetPlayerController 0)))
      (UserInterface|Viewport|AddtoViewport _returnvalue 0))))

(event EventTick
  (params (DeltaSeconds :type Float%20%28single-precision%29)))

(fn ConstructionScript)

(fn SpawnPlayers
  (params (Object :type Actor%20Object%20Reference))
  (bind _asplayer_start (Utilities|Casting|CastToPlayerStart Object))
  (if (== "P1" (Variables|/Script/Engine.PlayerStart|GetPlayerStartTag _asplayer_start))
    (bind _returnvalue (CallFunction|DetermineCharacterClass (Transformation|GetActorTransform Object) Object))
    (Variables|Default|Setplayer1 _returnvalue)
    (Pawn|Possess (Game|GetPlayerController 0) _returnvalue)
    (elif (== "P2" (Variables|/Script/Engine.PlayerStart|GetPlayerStartTag _asplayer_start))
      (bind _returnvalue_2 (CallFunction|DetermineCharacterClass (Transformation|GetActorTransform Object) Object))
      (bind _output_get (Variables|Default|Setplayer2 _returnvalue_2))
      (bind _returnvalue_3 (Class|GameplayStatics|CreatePlayer -1))
      (Pawn|Possess _returnvalue_3 _output_get))))

(fn DetermineCharacterClass
  (params (SpawnTransform :type Transform) (Owner :type Actor%20Object%20Reference))
  (bind _asbp_fggame_instance (Utilities|Casting|CastToBP_FGGameInstance (Game|GetGameInstance)))
  (switch Utilities|FlowControl|Switch|SwitchonECharacterClass (Variables|/Script/FighterGame.FGGameInstance|GetCharacterClass _asbp_fggame_instance)
    (:VE_Default
      (bind _returnvalue (Game|SpawnActorfromClass "/Game/Blueprints/BP_FGCharacterBase.BP_FGCharacterBase_C" SpawnTransform "Undefined" "MultiplyWithRoot" Owner 0))
      (return _returnvalue))
    (:VE_Mutant
      (bind _returnvalue_2 (Game|SpawnActorfromClass "/Game/Blueprints/BP_MutantCharacter.BP_MutantCharacter_C" SpawnTransform "Undefined" "MultiplyWithRoot" Owner 0))
      (return _returnvalue_2))))