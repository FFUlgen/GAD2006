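; Shared fighting-game camera that frames both players from a side-on offset.
; Shortly after BeginPlay it gets both players from BP_FGGameMode, spawns two BP_CameraEdge actors and places them once outside the players' starting positions, storing left and right limits.
; Each tick it follows a point between the players, with a weighted height, and zooms by scaling their horizontal separation into a clamped field of view.
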(event EventBeginPlay
  (Utilities|FlowControl|Delay 0.1)
  (bind _asbp_fggame_mode (Utilities|Casting|CastToBP_FGGameMode (Game|GetGameMode)))
  (Utilities|IsValid (Variables|/Script/FighterGame.FGGameModeBase|Getplayer1 _asbp_fggame_mode)
    (:Is%20Valid
      (Variables|Default|SetPlayer%201%20Ref (Variables|/Script/FighterGame.FGGameModeBase|Getplayer1 _asbp_fggame_mode))
      (Utilities|IsValid (Variables|/Script/FighterGame.FGGameModeBase|Getplayer2 _asbp_fggame_mode)
        (:Is%20Valid
          (Variables|Default|SetPlayer%202%20Ref (Variables|/Script/FighterGame.FGGameModeBase|Getplayer2 _asbp_fggame_mode))
          (bind _returnvalue (Game|SpawnActorfromClass "/Game/Blueprints/Functional/BP_CameraEdge.BP_CameraEdge_C" (Transformation|GetActorTransform) "Undefined" "MultiplyWithRoot" 0 0))
          (Variables|Default|SetLeftCameraEdge _returnvalue)
          (bind _returnvalue_2 (Game|SpawnActorfromClass "/Game/Blueprints/Functional/BP_CameraEdge.BP_CameraEdge_C" (Transformation|GetActorTransform) "Undefined" "MultiplyWithRoot" 0 0))
          (Variables|Default|SetRightCameraEdge _returnvalue_2)
          (CallFunction|SetCameraBoundaries))))))

(event EventTick
  (params (DeltaSeconds :type Float%20%28single-precision%29))
  (bind _player_1_ref (Variables|Default|GetPlayer%201%20Ref))
  (bind _player_2_ref (Variables|Default|GetPlayer%202%20Ref))
  (bind _returnvalue (Transformation|GetActorLocation _player_1_ref))
  (bind _returnvalue_2 (Transformation|GetActorLocation _player_2_ref))
  (bind (_x _y _z) (Math|Vector|BreakVector _returnvalue))
  (bind (_x_2 _y_2 _z_2) (Math|Vector|BreakVector _returnvalue_2))
  (if (and (Utilities|IsValid _player_1_ref) (Utilities|IsValid _player_2_ref))
    (Transformation|SetActorLocation (Math|Vector|MakeVector (/ (+ _x _x_2) 2.0) (+ (.Y (Math|Vector|BreakVector (Transformation|GetActorLocation (Variables|Default|GetPlayer%201%20Ref)))) 6.5e+02) (/ (+ _z _z_2) 1.7)) false false)
    (Camera|SetFieldOfView (Variables|CameraActor|GetCameraComponent) (Math|Float|Clamp(Float) (Math|Float|Absolute(Float) (* (- (.X (Math|Vector|BreakVector (Transformation|GetActorLocation (Variables|Default|GetPlayer%201%20Ref)))) (.X (Math|Vector|BreakVector (Transformation|GetActorLocation (Variables|Default|GetPlayer%202%20Ref))))) (Variables|Designer|GetLocationDifferenceMultiplier))) (Variables|Designer|GetFOV%20Min%20Clamp) (Variables|Designer|GetFOV%20Max%20Clamp)))))

(fn ConstructionScript)

(fn SetCameraBoundaries
  (bind _player_1_ref (Variables|Default|GetPlayer%201%20Ref))
  (bind _player_2_ref (Variables|Default|GetPlayer%202%20Ref))
  (bind _returnvalue (Transformation|GetActorLocation _player_2_ref))
  (bind _returnvalue_2 (Transformation|GetActorLocation _player_1_ref))
  (bind (_x _y _z) (Math|Vector|BreakVector _returnvalue))
  (bind (_x_2 _y_2 _z_2) (Math|Vector|BreakVector _returnvalue_2))
  (bind _returnvalue_3 (- _x -6e+02))
  (bind _returnvalue_4 (- _x_2 6e+02))
  (Variables|Default|SetLeftMax (- _returnvalue_4 4e+02))
  (Transformation|SetActorLocation (Variables|Default|GetLeftCameraEdge) (Math|Vector|MakeVector _returnvalue_4 _y_2 _z_2) false false)
  (Variables|Default|SetRightMax (- _returnvalue_3 -4e+02))
  (Transformation|SetActorLocation (Variables|Default|GetRightCameraEdge) (Math|Vector|MakeVector _returnvalue_3 _y _z) false false))