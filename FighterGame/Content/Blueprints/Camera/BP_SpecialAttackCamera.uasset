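; BP_SpecialAttackCamera is a camera that frames Player 1, by its name for special attack shots in a fighting game.
; After a short delay on BeginPlay, it caches both player references from BP_FGGameMode.
; Each Tick it snaps to a fixed world-space offset from Player 1 with a constant yaw and field of view, without interpolation.
; Player 2 is cached but never used, and activation of the camera is not handled here.
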(event EventBeginPlay
  (Utilities|FlowControl|Delay 0.03)
  (bind _asbp_fggame_mode (Utilities|Casting|CastToBP_FGGameMode (Game|GetGameMode)))
  (Utilities|IsValid (Variables|/Script/FighterGame.FGGameModeBase|Getplayer1 _asbp_fggame_mode)
    (:Is%20Valid
      (Variables|Default|SetPlayer%201%20Ref (Variables|/Script/FighterGame.FGGameModeBase|Getplayer1 _asbp_fggame_mode))
      (Utilities|IsValid (Variables|/Script/FighterGame.FGGameModeBase|Getplayer2 _asbp_fggame_mode)
        (:Is%20Valid
          (Variables|Default|SetPlayer%202%20Ref (Variables|/Script/FighterGame.FGGameModeBase|Getplayer2 _asbp_fggame_mode)))))))

(event EventTick
  (params (DeltaSeconds :type Float%20%28single-precision%29))
  (bind _player_1_ref (Variables|Default|GetPlayer%201%20Ref))
  (bind _returnvalue (Transformation|GetActorTransform _player_1_ref))
  (if (Utilities|IsValid (Variables|Default|GetPlayer%201%20Ref))
    (Transformation|SetActorTransform (Math|Transform|MakeTransform (Math|Vector|MakeVector (+ (.x (.location _returnvalue)) 1.6e+02) (+ (.y (.location _returnvalue)) 2.5e+02) (+ (.z (.location _returnvalue)) 15.0)) (Math|Rotator|MakeRotator 0.0 0.0 -1.2e+02) "1.000000,1.000000,1.000000"))
    (Camera|SetFieldOfView (Variables|CameraActor|GetCameraComponent) 75.0)))

(fn ConstructionScript)