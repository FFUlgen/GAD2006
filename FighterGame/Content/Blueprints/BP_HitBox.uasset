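; BP_HitBox is a fighting-game box actor that acts as a proximity box, strike or hurtbox for one of two players.
; SpawnHitbox colors the display mesh by type, moves it into place, shows it and immediately runs a single overlap check.
; CheckCollision uses the owner and game mode to pick the opponent, then tests their HurtBox.
; Proximity hits notify that player, while Strike hits pass damage, stun, block stun, pushback and launch.
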(event Custom|SpawnHitbox
  (switch Utilities|FlowControl|Switch|SwitchonEHitBox (Variables|Default|GetHitBoxType)
    (:HB_PROXIMITY
      (Rendering|Material|SetMaterial (Variables|Default|GetHitboxDisplay) 0 "/Game/Materials/Hitboxes/M_BasicColor_Yellow.M_BasicColor_Yellow"))
    (:HB_STRIKE
      (Rendering|Material|SetMaterial (Variables|Default|GetHitboxDisplay) 0 "/Game/Materials/Hitboxes/M_BasicColor_Red.M_BasicColor_Red"))
    (:HB_HURTBOX
      (Rendering|Material|SetMaterial (Variables|Default|GetHitboxDisplay) 0 "/Game/Materials/Hitboxes/M_BasicColor_Green.M_BasicColor_Green")))
  (Transformation|SetWorldLocation (Variables|Default|GetHitboxDisplay) (Variables|Default|GetHitBoxLocation) false false)
  (Rendering|SetVisibility (Variables|Default|GetHitboxDisplay) true false)
  (CallFunction|CheckCollision))

(event Custom|CheckCollision
  (bind _fggame_mode_base (Variables|Default|GetFGGame%20Mode%20Base))
  (bind _fggame_mode_base_2 (Variables|Default|GetFGGame%20Mode%20Base))
  (bind _player1 (Variables|/Script/FighterGame.FGGameModeBase|Getplayer1 _fggame_mode_base_2))
  (bind _player2 (Variables|/Script/FighterGame.FGGameModeBase|Getplayer2 _fggame_mode_base))
  ;[1 1 1] Check Collision
  (bind _isplayerone (CallFunction|DeterminePlayer))
  (if _isplayerone
    (if (Collision|IsOverlappingActor (Variables|/Script/FighterGame.FGCharacterBase|GetHurtBox _player2) :!class /Script/Engine.Actor)
      (switch Utilities|FlowControl|Switch|SwitchonEHitBox (Variables|Default|GetHitBoxType)
        (:HB_PROXIMITY
          (Class|FGCharacterBase|CollidedwithProximityHitbox _player2))
        (:HB_STRIKE
          (Class|FGCharacterBase|TakeDamage _player2 (Variables|Default|GetHitBoxDamage) (Variables|Default|GetHitStunTime) (Variables|Default|GetBlockStunTime) (Variables|Default|GetPushBackDistance) (Variables|Default|GetLaunchDistance)))))
    (elif (Collision|IsOverlappingActor (Variables|/Script/FighterGame.FGCharacterBase|GetHurtBox _player1) :!class /Script/Engine.Actor)
      (switch Utilities|FlowControl|Switch|SwitchonEHitBox (Variables|Default|GetHitBoxType)
        (:HB_PROXIMITY
          (Class|FGCharacterBase|CollidedwithProximityHitbox _player1))
        (:HB_STRIKE
          (Class|FGCharacterBase|TakeDamage _player1 (Variables|Default|GetHitBoxDamage) (Variables|Default|GetHitStunTime) (Variables|Default|GetBlockStunTime) (Variables|Default|GetPushBackDistance) (Variables|Default|GetLaunchDistance)))))))

(fn ConstructionScript)

(fn DeterminePlayer
  (bind _asfggame_mode_base (Utilities|Casting|CastToFGGameModeBase (Game|GetGameMode)))
  (bind _output_get (Variables|Default|SetFGGame%20Mode%20Base _asfggame_mode_base))
  (if (== (Variables|/Script/FighterGame.FGGameModeBase|Getplayer1 _output_get) (Components|GetOwner))
    (return true)
    (else
      (return false))))